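; BP_InfiniteTerrainGameMode is a game mode that builds a chained, tile-based infinite terrain and keeps the score.
; On BeginPlay it fills a pool of nav mesh bounds volumes and spawns the opening tiles.
; Each new BP_Tile receives that pool, spawns its props, and supplies the attach location used as the next tile's transform.
; NewTileConquered increments the score, which GetScore returns.
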(event `self.ReceiveBeginPlay`
  (`self.PopulateBoundsVolumePool`)
  (for _ (range 3)
    (`self.SpawnTile`)))

(fn `GetScore`
  (returns (Score :type Integer))
  (return (`self.Score`)))

(fn `NewTileConquered`
  (`/Engine/EditorBlueprintResources/StandardMacros.IncrementInt` (`self.Score`)))

(fn `SpawnTile`
  (bind _returnvalue (`|SpawnActorFromClass` "/Game/Dynamic/Terrain/Tile/BP_Tile.BP_Tile_C" (`self.NextTileTransform`) "Undefined" "OverrideRootScale"))
  (`TileController.SetPool` _returnvalue (`self.NavMeshBoundsVolumePool`))
  (`/Game/Dynamic/Terrain/Tile/BP_Tile.SpawnProps` _returnvalue)
  (bind _attachtransform (`/Game/Dynamic/Terrain/Tile/BP_Tile.GetAttachLocation` _returnvalue))
  (set `self.NextTileTransform` _attachtransform))

(fn `UserConstructionScript`)